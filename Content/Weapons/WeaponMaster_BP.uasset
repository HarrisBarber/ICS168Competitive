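; Master weapon actor that attaches to its owning pawn's hand socket and fires hitscan shots from the follow camera.
; The server fire event loops on a delay while firing and aiming down sights, tracing for objects, spawning an impact effect and applying damage.
; StartFire instead runs a single CameraAim trace on authority, while remote callers forward to the server.
; An owner OnRep completes deferred attachment on clients.
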(event `Server_StartFire`
  (bind _owningpawn (`self.OwningPawn`))
  (bind _followcamera (`/Game/ThirdPersonBP/Blueprints/ThirdPersonCharacter.FollowCamera` _owningpawn))
  (bind _returnvalue (`SceneComponent.K2_GetComponentLocation` _followcamera))
  (set `self.isFiring` true)
  (if (`self.IsLoaded`) :!label _label
    (if (and (`self.isFiring`) (`/Game/ThirdPersonBP/Blueprints/ThirdPersonCharacter.isPlayerADS` _owningpawn))
      (set `self.IsLoaded` false)
      (bind _outhit (`KismetSystemLibrary.LineTraceSingleForObjects` _returnvalue (+ _returnvalue (* (`SceneComponent.GetForwardVector` _followcamera) 1000000.0)) (`|MakeArray` "ObjectTypeQuery3" "ObjectTypeQuery1" :!type "EObjectTypeQuery Enum") false (`|MakeArray` (`self.OwningPawn`))))
      (bind (_bblockinghit _binitialoverlap _time _distance _location _impactpoint _normal _impactnormal _physmat _hitactor) (`GameplayStatics.BreakHitResult` _outhit))
      (`self.DisplayImpactEffect` _location)
      (`self.DealDamage` _hitactor 10.0)
      (`KismetSystemLibrary.Delay` (`self.FireDelay`))
      (set `self.IsLoaded` true)
      (goto _label))))

(event `Server_StopFire`
  (set `self.isFiring` false))

(event `DealDamage`
  (params (damagedActor :type "Actor Object Reference") (damage :type "Float (double-precision)"))
  (`GameplayStatics.ApplyDamage` damagedActor damage))

(event `DisplayImpactEffect`
  (params (location :type "Vector Structure"))
  (`GameplayStatics.SpawnEmitterAtLocation` "/Game/InfinityBladeEffects/Effects/FX_Monsters/FX_Monster_Ausar/P_AU_Shieldslam_Impact.P_AU_Shieldslam_Impact" location))

(fn `AttachToOwner`
  (bind _owningpawn (`self.OwningPawn`))
  (`/Engine/EditorBlueprintResources/StandardMacros.IsValid` _owningpawn
    (:`Is Valid`
      (`SceneComponent.K2_AttachToComponent` (`self.WeaponMesh`) (`Character.Mesh` _owningpawn) (`/Game/ThirdPersonBP/Blueprints/ThirdPersonCharacter.RHand_WeaponSocket` _owningpawn) "KeepRelative" "KeepRelative" "KeepWorld" true)
      (set `/Game/ThirdPersonBP/Blueprints/ThirdPersonCharacter.EquippedWeapon` self _owningpawn))
    (:`Is Not Valid`
      (set `self.NeedsAttachedUpdateOnOwnerRep` true))))

(fn `CameraAim`
  (bind _owningpawn (`self.OwningPawn`))
  (bind _followcamera (`/Game/ThirdPersonBP/Blueprints/ThirdPersonCharacter.FollowCamera` _owningpawn))
  ;[1 1 1] Aim and Shoot
  (bind _output_get (`self.ViewPoint`))
  (bind _outaim1 (`self.GetAimVector`))
  (bind _muzzlelocation (`self.GetMuzzleLocation`))
  (set `self.AimVector` (`KismetMathLibrary.GetForwardVector` (`Pawn.GetBaseAimRotation` _owningpawn)))
  (bind _returnvalue (+ _output_get (* _outaim1 100000)))
  (bind _outhit (`KismetSystemLibrary.LineTraceSingle` (+ (* (`SceneComponent.GetForwardVector` _followcamera) 150.0) (`SceneComponent.K2_GetComponentLocation` _followcamera)) _returnvalue "TraceTypeQuery1"))
  (bind (_bblockinghit _binitialoverlap _time _distance _location _impactpoint _normal _impactnormal _physmat _hitactor) (`GameplayStatics.BreakHitResult` _outhit))
  (set `self.AimVector` (`KismetMathLibrary.SelectVector` _location (- _returnvalue _muzzlelocation) _bblockinghit))
  ;[1 1 1] Deal Damage
  (`/Engine/EditorBlueprintResources/StandardMacros.IsValid` _hitactor
    (:`Is Valid`
      (bind _asthird_person_character (cast `/Game/ThirdPersonBP/Blueprints/ThirdPersonCharacter` _hitactor))
      (`GameplayStatics.ApplyDamage` _asthird_person_character 10.0)
      (return))))

(fn `GetAimVector`
  (returns (OutAim1 :type "Vector Structure"))
  (locals (OutAim :type "Vector Structure"))
  (bind _owningpawn (`self.OwningPawn`))
  (`/Engine/EditorBlueprintResources/StandardMacros.IsValid` _owningpawn
    (:`Is Valid`
      (set `local.OutAim` (`KismetMathLibrary.GetForwardVector` (`Pawn.GetBaseAimRotation` _owningpawn))))
    (:`Is Not Valid`
      (set `local.OutAim` (`KismetMathLibrary.Conv_RotatorToVector` (`Pawn.GetControlRotation` _owningpawn)))))
  (return (`local.OutAim`)))

(fn `GetMuzzleLocation`
  (returns (MuzzleLocation :type "Vector Structure"))
  (return (`SceneComponent.GetSocketLocation` (`self.WeaponMesh`) (`self.MuzzleSocket`))))

(fn `OnRep_OwningPawn`
  (bind _owningpawn (`self.OwningPawn`))
  (if (and (`self.NeedsAttachedUpdateOnOwnerRep`) (`KismetSystemLibrary.IsValid` (`self.OwningPawn`)))
    (set `self.NeedsAttachedUpdateOnOwnerRep` false)
    (`/Engine/EditorBlueprintResources/ActorMacros.Switch Has Authority`
      (:`Remote`
        (if (== (`/Game/ThirdPersonBP/Blueprints/ThirdPersonCharacter.EquippedWeapon` _owningpawn) self)
          _
          (elif (`/Game/ThirdPersonBP/Blueprints/ThirdPersonCharacter.CanFire` _owningpawn)
            (`self.AttachToOwner`)))))))

(fn `SetOwningPawn`
  (params (`Owning Pawn` :type "/Game/ThirdPersonBP/Blueprints/ThirdPersonCharacter Object Reference"))
  (if (!= `Owning Pawn` (`self.OwningPawn`))
    (bind _output_get (set `self.OwningPawn` `Owning Pawn`))
    (`self.SetOwner` _output_get)))

(fn `StartFire`
  (`/Engine/EditorBlueprintResources/ActorMacros.Switch Has Authority`
    (:`Authority`
      (if (not (`self.PressedFire`))
        (set `self.PressedFire` true)
        (`self.CameraAim`)
        (`GameplayStatics.SpawnEmitterAtLocation` "/Game/InfinityBladeEffects/Effects/FX_Monsters/FX_Monster_Ausar/P_AU_Shieldslam_Impact.P_AU_Shieldslam_Impact" (`self.AimVector`))))
    (:`Remote`
      (`self.Server_StartFire`))))

(fn `StopFire`
  (`/Engine/EditorBlueprintResources/ActorMacros.Switch Has Authority`
    (:`Authority`
      _)
    (:`Remote`
      (`self.Server_StopFire`)))
  (if (`self.PressedFire`)
    (set `self.PressedFire` false)))

(fn `UserConstructionScript`)

(fn `ViewPoint`
  (returns (Output_Get :type "Vector Structure"))
  (set `self.OutViewLocation` (0.0 0.0 0.0))
  (bind _desiredview (`CameraComponent.GetCameraView` (`/Game/ThirdPersonBP/Blueprints/ThirdPersonCharacter.FollowCamera` (`self.OwningPawn`)) 0.0))
  (bind _output_get (set `self.OutViewLocation` (break `MinimalViewInfo` _desiredview)))
  (return _output_get))